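; BP_Rocket is the rocket actor's presentation layer, handling thruster effects, crash and victory feedback.
; Each tick it toggles the main, left and right thruster trails from their state flags and fades one lazily spawned, attached engine sound in or out.
; Crashing spawns an effect, swaps to a destroyed mesh and plays a sound.
; Victory plays VFX and sound, then marks the level complete and saves through GI_Rocket.
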(event EventTick
  (params (DeltaSeconds :type Float%20%28single-precision%29))
  ;[0.15 0.097 0.02415 0.5] Thruster particle Management  (OnTick)
  (Utilities|FlowControl|Sequence
    (:then_0
      (CallFunction|ManageThrusterVFX (Variables|Default|GetMainThrusterTrail) (Variables|Default|GetIsUsingMainThruster))
      (CallFunction|ManageEngineSFX))
    (:then_1
      (CallFunction|ManageThrusterVFX (Variables|Default|GetLeftThrusterTrail) (Variables|Default|GetIsUsingLeftThruster))
      (CallFunction|ManageEngineSFX))
    (:then_2
      (CallFunction|ManageThrusterVFX (Variables|Default|GetRightThrusterTrail) (Variables|Default|GetIsUsingRightThruster))
      (CallFunction|ManageEngineSFX))))

(event EventPlayCrashFrontEndEvents
  ;[1 0.1309 0.1668] CrashEvents
  (Utilities|FlowControl|Sequence
    (:then_0
      (Niagara|SpawnSystematLocation "/Game/Free_Magic/VFX_Niagara/NS_Free_Magic_Hit1.NS_Free_Magic_Hit1" (Transformation|GetActorLocation)))
    (:then_1
      (Components|StaticMesh|SetStaticMesh (Variables|Default|GetStaticMesh) (Variables|Default|GetDestroyedMesh)))
    (:then_2
      (Audio|PlaySound2D "/Game/Audio/Crash/MS_Crash.MS_Crash" 1.0 1.0 0.0 0 0))))

(event EventPlayVictoryFrontEndEvents
  ;[0.1297 0.599 0.1164] VictoryEvents
  (Niagara|SpawnSystematLocation "/Game/VFX/NS_VictoryVFX.NS_VictoryVFX" (Transformation|GetActorLocation))
  (Audio|PlaySound2D "/Game/Audio/Victory/MS_Victory.MS_Victory" 1.0 1.0 0.0 0 0)
  (bind _asgi_rocket (Utilities|Casting|CastToGI_Rocket (Game|GetGameInstance)))
  (bind _returnvalue (Game|GetCurrentLevelName true))
  (Default|MarkLevelasComplete _asgi_rocket (Utilities|String|StringToName _returnvalue))
  (Default|SaveLevelSettings _asgi_rocket))

(fn ConstructionScript)

(fn ManageThrusterVFX
  (params (ThrusterTrail :type Actor%20Component%20Object%20Reference) (ThrusterState :type Boolean))
  (if ThrusterState
    (Components|Activation|Activate ThrusterTrail false)
    (else
      (Components|Activation|Deactivate ThrusterTrail))))

(fn ManageEngineSFX
  (if (Math|Boolean|ORBoolean (Variables|Default|GetIsUsingMainThruster) (Variables|Default|GetIsUsingLeftThruster) (Variables|Default|GetIsUsingRightThruster))
    (bind _enginesoundsource (Variables|Rocket|GetEngineSoundSource)
      (:then
        (if (not (Audio|Components|Audio|IsPlaying _enginesoundsource))
          (Audio|Components|Audio|FadeIn (Variables|Rocket|GetEngineSoundSource) 0.2 1.0 0.0 "Linear" :!class /Script/Engine.AudioComponent)))
      (:else
        (bind _returnvalue (Audio|SpawnSoundAttached "/Game/Audio/Engine/MS_MainEngine.MS_MainEngine" (Variables|Default|GetStaticMesh) "None" "0, 0, 0" "0, 0, 0" "KeepRelativeOffset" false 1.0 1.0 0.0 0 0 false))
        (bind _output_get (Variables|Rocket|SetEngineSoundSource _returnvalue))
        (Audio|Components|Audio|FadeIn _output_get 0.2 1.0 0.0 "Linear" :!class /Script/Engine.AudioComponent)))
    (else
      (bind _enginesoundsource_2 (Variables|Rocket|GetEngineSoundSource)
        (:then
          (if (Audio|Components|Audio|IsPlaying _enginesoundsource_2)
            (Audio|Components|Audio|FadeOut (Variables|Rocket|GetEngineSoundSource) 0.1 0.0 "Linear" :!class /Script/Engine.AudioComponent)))
        (:else)))))