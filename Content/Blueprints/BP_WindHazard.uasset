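; Wind trap hazard Blueprint that handles the front-end visuals of a fan as the trap toggles on and off.
; On activation, a looping timer drives the fan's stepped local rotation and the wind FX activates; on stop, the timer is cleared and the FX deactivates.
; No wind force or gameplay effect is implemented in this graph, and a debug box draw is left disconnected.
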(event Custom|Spin%20Fan
  ;[0.137 0.15 0.07151 0.5] Activate Fan Spin Visual
  (Transformation|AddLocalRotation (Variables|Default|Getfan) "0.000000,0.000000,30.000000" false false))

(event EventPlayFrontEndTrapActivatedEvents
  ;[0.137 0.15 0.07151 0.5] Activate Fan Spin Visual
  (bind _returnvalue (Utilities|Time|SetTimerbyEvent (EventDispatchers|CreateEvent :!event Custom|Spin%20Fan) (Variables|Default|GetFanSpinInterval) true))
  (Variables|Default|SetFanSpinnerTImerHandle _returnvalue)
  (Components|Activation|Activate (Variables|Default|GetWindFX) false))

(event EventStopFrontEndTrapActivatedEvents
  ;[0.137 0.15 0.07151 0.5] Stop Fan Spin
  (Utilities|Time|ClearandInvalidateTimerbyHandle (Variables|Default|GetFanSpinnerTImerHandle))
  (Components|Activation|Deactivate (Variables|Default|GetWindFX)))

(fn ConstructionScript)