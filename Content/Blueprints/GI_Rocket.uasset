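; Game instance for a rocket game that tracks which levels are cleared and persists that progress in a save slot.
; On Init it loads or creates a BP_LevelSettings save object and copies its LevelTracking array into the instance.
; MarkLevelAsComplete flags a matching uncleared entry or adds a cleared one, labeled from CurrentLevel.
; SaveLevelSettings separately writes the array back to the slot.
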(event EventInit
  (|CallParentFunction)
  (CallFunction|ManageDefaultSettings))

(fn MarkLevelasComplete
  (params (LevelName :type Name))
  (bind _leveltracking (Variables|Default|GetLevelTracking))
  (if (Utilities|Array|ContainsItem (Variables|Default|GetLevelTracking) (Utilities|Struct|MakeLvlTrackerStruct LevelName false (CallFunction|MakeLevelName)))
    (Utilities|Array|SetArrayElem _leveltracking (Utilities|Array|FindItem _leveltracking (Utilities|Struct|MakeLvlTrackerStruct LevelName false (CallFunction|MakeLevelName))) (Utilities|Struct|MakeLvlTrackerStruct LevelName true (CallFunction|MakeLevelName)))
    (else
      (Utilities|Array|AddUnique (Variables|Default|GetLevelTracking) (Utilities|Struct|MakeLvlTrackerStruct LevelName true (CallFunction|MakeLevelName))))))

(fn ManageDefaultSettings
  (bind _returnvalue (SaveGame|DoesSaveGameExist (Variables|Default|GetLevelSettingsName)))
  (if _returnvalue
    (bind _returnvalue_2 (SaveGame|LoadGamefromSlot (Variables|Default|GetLevelSettingsName)))
    (bind _levelsettings (Variables|Default|GetLevelSettings)
      (:then
        (CallFunction|LoadLevelSettings _levelsettings))
      (:else
        (bind _asbp_level_settings (Utilities|Casting|CastToBP_LevelSettings _returnvalue_2))
        (bind _output_get (Variables|Default|SetLevelSettings _asbp_level_settings))
        (CallFunction|LoadLevelSettings _output_get)))
    (else
      (bind _returnvalue_3 (SaveGame|CreateSaveGameObject "/Game/Blueprints/BP_LevelSettings.BP_LevelSettings_C"))
      (bind _output_get_2 (Variables|Default|SetLevelSettings _returnvalue_3))
      (CallFunction|LoadLevelSettings _output_get_2))))

(fn LoadLevelSettings
  (params (LevelSettings :type BP%20Level%20Settings%20Object%20Reference))
  (bind _output_get (Variables|Default|SetLevelTracking (Variables|/Game/Blueprints/BP_LevelSettings.BP_LevelSettings_C|GetLevelTracking LevelSettings)))
  (if (Utilities|Array|IsEmpty _output_get)
    (Development|PrintString "Empty")))

(fn SaveLevelSettings
  (bind _levelsettings (Variables|Default|GetLevelSettings))
  (Variables|/Game/Blueprints/BP_LevelSettings.BP_LevelSettings_C|SetLevelTracking _levelsettings (Variables|Default|GetLevelTracking))
  (SaveGame|SaveGametoSlot _levelsettings (Variables|Default|GetLevelSettingsName)))

(fn MakeLevelName
  (return (Utilities|String|Append "Level " (Utilities|String|ToString(Integer) (Variables|Default|GetCurrentLevel)))))